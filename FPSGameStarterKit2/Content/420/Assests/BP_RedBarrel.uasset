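; BP_RedBarrel is an explosive physics barrel that blows up shortly after taking damage.
; Its Cylinder simulates physics from BeginPlay, and any damage activates the attached particle system as a short fuse.
; After a delay, it spawns a BP_Explosion at the cylinder's current transform, passing effect, sound, force and damage settings with itself as ignored actor, then destroys itself.
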(event `self.ReceiveBeginPlay`
  (`PrimitiveComponent.SetSimulatePhysics` (`self.Cylinder`) true))

(event `self.ReceiveAnyDamage`
  (params (Damage :type "Float (single-precision)") (DamageType :type "DamageType Object Reference") (InstigatedBy :type "Controller Object Reference") (DamageCauser :type "Actor Object Reference"))
  (`ActorComponent.Activate` (`self.ParticleSystem`) false)
  (`KismetSystemLibrary.Delay` 2.0)
  (`|SpawnActorFromClass` "/Game/FPS_Game/Blueprints/Weapons/Base/BP_Explosion.BP_Explosion_C" (`SceneComponent.K2_GetComponentToWorld` (`self.Cylinder`)) "AlwaysSpawn" "OverrideRootScale" null "/Game/FPS_Game/Particles/P_Explosion_Big.P_Explosion_Big" "/Game/FPS_Game/Sounds/SFX/Weapon_SFX/Explosion_Cue.Explosion_Cue" 800.0 500.0 0.2 self null null)
  (`self.K2_DestroyActor`))

(fn `UserConstructionScript`)