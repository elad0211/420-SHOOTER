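; Shotgun weapon child Blueprint that reloads one round per reload call.
; Begin play, interaction and firing defer to the parent, while ReloadWeapon replaces the parent logic and Reload is left empty.
; Reloading blocks firing, plays first- and third-person montages, and waits out the first-person one.
; It then moves one round from reserve and re-enables firing, both only if reserve exceeds one.
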(event `self.ReceiveBeginPlay`
  ;[1 1 1] These events call the logic from the parent class
  (`parent.ReceiveBeginPlay`))

(event `/Game/FPS_Game/Blueprints/System/BPI_Interact.BPI_Interaction`
  (params (CharacterReference :type "/Game/FPS_Game/Blueprints/BP_CharacterBase Object Reference"))
  ;[1 1 1] These events call the logic from the parent class
  (`parent.BPI_Interaction` CharacterReference))

(event `self.WeaponFire`
  ;[1 1 1] These events call the logic from the parent class
  (`parent.WeaponFire`))

(event `self.ReloadWeapon`
  (bind _playercast (`self.PlayerCast`))
  ;[1 1 1] These events don't call the parent class logic
  ;[1 1 1] Custom reload logic for this weapon child class so that it reloads only 1 button at a time
  (if (< (`self.AmmoCurrent`) (`self.AmmoMax`))
    (if (`self.CanFire`)
      (set `self.CanFire` false)
      (`|ExecutionSequence`
        (:`then_0`
          ;;[1 1 1] Anim montage goes here
          (bind _returnvalue (`AnimInstance.Montage_Play` (`SkeletalMeshComponent.GetAnimInstance` (`/Game/FPS_Game/Blueprints/BP_CharacterBase.Mesh_FPP` _playercast)) "/Game/FPS_Game/Character/UE5_Retargeting/Mannequins/Animations/Retarget_Anims_FPP/UE5_FPP_Rifle_Pull_Down_Montage.UE5_FPP_Rifle_Pull_Down_Montage" 1.0 "Duration" 0.0 true)) ; FPP
          (`KismetSystemLibrary.Delay` _returnvalue)
          (if (> (`self.AmmoInReserve`) 1)
            (set `self.AmmoCurrent` (`KismetMathLibrary.Clamp` (+ (`self.AmmoCurrent`) 1) 0 (`self.AmmoMax`)))
            (set `self.AmmoInReserve` (- (`self.AmmoInReserve`) 1))
            (set `self.CanFire` true)))
        (:`then_1`
          (`AnimInstance.Montage_Play` (`SkeletalMeshComponent.GetAnimInstance` (`Character.Mesh` _playercast)) "/Game/FPS_Game/Character/UE5_Retargeting/Mannequins/Animations/Retarget_Anims/UE5_Equip_Rifle_Standing_Montage.UE5_Equip_Rifle_Standing_Montage" 1.0 "Duration" 0.0 true) ; TPP
        )))))

(event `self.Reload`
  ;[1 1 1] These events don't call the parent class logic
)

(fn `UserConstructionScript`
  (`parent.UserConstructionScript`))